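; BP_CrossingRoad is a road crossing actor that hooks up its four traffic lights to a shared traffic controller.
; Four child actor components, named for 0, 90, 180 and 270 degree orientations, hold the lights.
; On BeginPlay, a helper function passes each spawned child actor to TrafficController through AddTrafficLightActor.
; The construction script is empty, and the Blueprint itself contains no light-switching logic.
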(event EventBeginPlay
  ;[1 1 1] Init Traffic Controller
  (CallFunction|StartTrafficChild (Variables|Default|GetTrafficLightBP%200))
  (CallFunction|StartTrafficChild (Variables|Default|GetTrafficLightBP%2090))
  (CallFunction|StartTrafficChild (Variables|Default|GetTrafficLightBP%20180))
  (CallFunction|StartTrafficChild (Variables|Default|GetTrafficLightBP%20270)))

(fn ConstructionScript)

(fn StartTrafficChild
  (params (NewParam :type Child%20Actor%20Component%20Object%20Reference))
  (Class|TrafficController|AddTrafficLightActor (Variables|Default|GetTrafficController) (Variables|/Script/Engine.ChildActorComponent|GetChildActor NewParam))
  (return))