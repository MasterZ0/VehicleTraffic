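; Road spline actor that builds a road from spline mesh segments along its Spline in the construction script.
; The script calls DrawSpline for each consecutive point pair, which adds a spline mesh component, copies both points' local locations and tangents, and attaches it to the root.
; When the spline is not a closed loop, an extra segment runs from the point-count index back to the first point.
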(fn ConstructionScript
  (bind _spline (Variables|Default|GetSpline))
  (bind _returnvalue (Spline|GetNumberOfSplinePoints _spline))
  ;[1 1 1] Get Spline indexs and Draw Static Mesh
  (for _index (range 0 (- _returnvalue 2))
    (CallFunction|DrawSpline _index (+ _index 1)))
  (if (not (Class|SplineComponent|IsClosedLoop _spline)) ; TODO: Get Validate event
    (CallFunction|DrawSpline _returnvalue)))

(fn DrawSpline
  (params (StartIndex :type Integer) (EndIndex :type Integer))
  (bind _spline (Variables|Default|GetSpline))
  (bind (_location _tangent) (Spline|GetLocationandTangentatSplinePoint _spline EndIndex "Local"))
  (bind (_location_2 _tangent_2) (Spline|GetLocationandTangentatSplinePoint _spline StartIndex "Local"))
  (bind _returnvalue (AddComponent|AddSplineMeshComponent false)) ; Get mesh and add component\nReview: Physic Trigger
  (SplineMesh|SetStartandEnd _returnvalue _location_2 _tangent_2 _location _tangent true :!class /Script/Engine.SplineMeshComponent)
  (Transformation|AttachComponentToComponent _returnvalue (Variables|Default|GetDefaultSceneRoot) "None" "KeepRelative" "KeepRelative" "KeepRelative" true))