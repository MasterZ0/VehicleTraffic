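; Vehicle base Blueprint that handles drift zone detection and trail effects, and links the car to its widget.
; On BeginPlay it registers itself as the owner of its WBP_Car widget.
; A detector component responds to actors implementing the Drift interface by calling enter and exit drift zone functions.
; Left and right socket-based trails start after a short delay on entry and end on exit.
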(event OnComponentBeginOverlap(DriftZoneDetector2)
  (params (OverlappedComponent :type Primitive%20Component%20Object%20Reference) (OtherActor :type Actor%20Object%20Reference) (OtherComp :type Primitive%20Component%20Object%20Reference) (OtherBodyIndex :type Integer) (bFromSweep :type Boolean) (SweepResult :type Hit%20Result%20Structure%20%28by%20ref%29))
  ;[1 1 1] Drift Trigger
  (if (Utilities|DoesObjectImplementInterface OtherActor "/Script/VehicleTraffic.Drift")
    (Default|CallEnterDriftZone)
    ;[1 1 1] Trail Effect
    (Utilities|FlowControl|Delay 0.4)
    (Effects|Particles|Trails|BeginTrails (Variables|Default|GetLeft) "TrailLeftStart" "TrailLeftEnd" "ETrailWidthMode_FromCentre" 4.0)
    (Effects|Particles|Trails|BeginTrails (Variables|Default|GetRight) "TrailRightStart" "TrailRightEnd" "ETrailWidthMode_FromCentre" 4.0)))

(event OnComponentEndOverlap(DriftZoneDetector2)
  (params (OverlappedComponent :type Primitive%20Component%20Object%20Reference) (OtherActor :type Actor%20Object%20Reference) (OtherComp :type Primitive%20Component%20Object%20Reference) (OtherBodyIndex :type Integer))
  ;[1 1 1] Drift Trigger
  (if (Utilities|DoesObjectImplementInterface OtherActor "/Script/VehicleTraffic.Drift")
    (Default|CallExitDriftZone)
    ;[1 1 1] Trail Effect
    (Effects|Particles|Trails|EndTrails (Variables|Default|GetLeft))
    (Effects|Particles|Trails|EndTrails (Variables|Default|GetRight))))

(event EventBeginPlay
  ;[1 1 1] Widget
  (bind _aswbp_car (Utilities|Casting|CastToWBP_Car (Variables|Default|GetWidgetInstance)))
  (Variables|/Game/Blueprints/Car/WBP_Car.WBP_Car_C|SetVehicleOwner _aswbp_car self))

(fn ConstructionScript)