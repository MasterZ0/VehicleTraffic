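; VehicleBaseBP is a base car Blueprint that links the vehicle to its UI and reacts to drift zones.
; On BeginPlay it sets itself as VehicleOwner on its Car_UI widget instance.
; DriftZoneDetector overlaps with actors implementing the Drift interface trigger enter and exit drift zone calls.
; Entering also starts socket-based Left and Right trails after a short delay, and exiting ends them immediately.
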(event OnComponentBeginOverlap(DriftZoneDetector)
  (params (OverlappedComponent :type Primitive%20Component%20Object%20Reference) (OtherActor :type Actor%20Object%20Reference) (OtherComp :type Primitive%20Component%20Object%20Reference) (OtherBodyIndex :type Integer) (bFromSweep :type Boolean) (SweepResult :type Hit%20Result%20Structure%20%28by%20ref%29))
  ;[1 1 1] Drift Trigger
  (if (Utilities|DoesObjectImplementInterface OtherActor "/Script/VehicleTraffic.Drift")
    (Default|CallEnterDriftZone)
    ;[1 1 1] Trail Effect
    (Utilities|FlowControl|Delay 0.4)
    (Effects|Particles|Trails|BeginTrails (Variables|Default|GetLeft) "TrailLeftStart" "TrailLeftEnd" "ETrailWidthMode_FromCentre" 4.0)
    (Effects|Particles|Trails|BeginTrails (Variables|Default|GetRight) "TrailRightStart" "TrailRightEnd" "ETrailWidthMode_FromCentre" 4.0)))

(event OnComponentEndOverlap(DriftZoneDetector)
  (params (OverlappedComponent :type Primitive%20Component%20Object%20Reference) (OtherActor :type Actor%20Object%20Reference) (OtherComp :type Primitive%20Component%20Object%20Reference) (OtherBodyIndex :type Integer))
  ;[1 1 1] Drift Trigger
  (if (Utilities|DoesObjectImplementInterface OtherActor "/Script/VehicleTraffic.Drift")
    (Default|CallExitDriftZone)
    ;[1 1 1] Trail Effect
    (Effects|Particles|Trails|EndTrails (Variables|Default|GetLeft))
    (Effects|Particles|Trails|EndTrails (Variables|Default|GetRight))))

(event EventBeginPlay
  ;[1 1 1] Widget
  (bind _ascar_ui (Utilities|Casting|CastToCar_UI (Variables|Default|GetWidgetInstance)))
  (Variables|/Game/Blueprints/Car/Car_UI.Car_UI_C|SetVehicleOwner _ascar_ui self))

(fn ConstructionScript)