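; Behavior tree task that initializes an AI car by finding the road spline it sits on.
; It takes the first RoadSpline actor overlapping the Car_AIController's RoadDetector and writes its spline to the blackboard.
; It succeeds when that spline is valid and prints an error and fails when it is not.
; A failed cast stops execution without finishing the task.
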(event EventReceiveExecuteAI
  (params (OwnerController :type AI%20Controller%20Object%20Reference) (ControlledPawn :type Pawn%20Object%20Reference))
  (bind _ascar_aicontroller (Utilities|Casting|CastToCar_AIController OwnerController))
  (bind _asroad_spline (Utilities|Casting|CastToRoadSpline (Utilities|Array|Get(acopy) (Collision|GetOverlappingActors (Variables|/Game/Blueprints/Car/CarAI/Car_AIController.Car_AIController_C|GetRoadDetector _ascar_aicontroller) "/Game/Blueprints/Road/RoadSpline.RoadSpline_C" :!class /Script/Engine.PrimitiveComponent))))
  (Utilities|IsValid (Variables|/Game/Blueprints/Road/RoadSpline.RoadSpline_C|GetSpline _asroad_spline)
    (:Is%20Valid
      (Class|BTFunctionLibrary|SetBlackboardValueasObject (Variables|Default|GetSpline) (Variables|/Game/Blueprints/Road/RoadSpline.RoadSpline_C|GetSpline _asroad_spline))
      (AI|BehaviorTree|FinishExecute true))
    (:Is%20Not%20Valid
      (Development|PrintString "InitCar: Cast Failure")
      (AI|BehaviorTree|FinishExecute false))))