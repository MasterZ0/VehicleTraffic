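; FollowSplineBP is a behavior tree task that moves an AI pawn along a spline.
; On execute it calls GetPathDirection with the spline and the controller's transform, without using a returned value.
; Each tick, FollowPath advances the stored distance from speed, delta time, offset and direction, and the pawn's transform is set directly to the result.
; The task never calls Finish Execute in this graph.
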(event EventReceiveExecuteAI
  (params (OwnerController :type AI%20Controller%20Object%20Reference) (ControlledPawn :type Pawn%20Object%20Reference))
  (bind _returnvalue (Transformation|GetActorTransform OwnerController))
  (Class|SplineLibrary|GetPathDirection (Variables|Default|GetSpline) (.location _returnvalue) (.rotation _returnvalue)))

(event EventReceiveTickAI
  (params (OwnerController :type AI%20Controller%20Object%20Reference) (ControlledPawn :type Pawn%20Object%20Reference) (DeltaSeconds :type Float%20%28single-precision%29))
  (bind (_outposition _outrotation _newdistance) (Class|SplineLibrary|FollowPath (Variables|Default|GetSpline) (Variables|Default|GetOffset) (Variables|Default|GetSpeed) (Variables|Default|GetDistance) (Utilities|Time|GetWorldDeltaSeconds) (Variables|Default|GetInverseDirection)))
  (Variables|Default|SetDistance _newdistance)
  (Transformation|SetActorTransform ControlledPawn (Math|Transform|MakeTransform _outposition _outrotation "1,1,1")))